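; BP_Car is a drivable car Blueprint that moves a physics-driven Cube with simple steering and drift.
; Each Tick yaws the Cube by InputDirection and TurnSpeed, scaled by delta time.
; It then blends forward thrust from Acceleration with current velocity by DriftAmount, adds the current velocity again, and sets the result as linear velocity.
; InputDirection is only read here, never set.
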(event `self.ReceiveTick`
  (params (DeltaSeconds :type "Float (single-precision)"))
  (bind _cube (`self.Cube`))
  (bind _cube_2 (`self.Cube`))
  (bind _output_get (set `self.MoveSpeed` (* DeltaSeconds (`self.Acceleration`))))
  (`SceneComponent.K2_AddLocalRotation` _cube_2 (`KismetMathLibrary.MakeRotator` 0.0 0.0 (* (`self.InputDirection`) (`self.TurnSpeed`) DeltaSeconds)) false false)
  (bind _returnvalue (`PrimitiveComponent.GetPhysicsLinearVelocity` _cube "None"))
  (`PrimitiveComponent.SetPhysicsLinearVelocity` _cube (+ (`KismetMathLibrary.VLerp` (* (`SceneComponent.GetForwardVector` _cube_2) _output_get) _returnvalue (`self.DriftAmount`)) _returnvalue) false "None"))

(fn `UserConstructionScript`)