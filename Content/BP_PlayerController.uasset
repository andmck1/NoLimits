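; Player controller for a car game that turns Enhanced Input actions into steering for the car and shows the HUD.
; On BeginPlay it adds the car input mapping context, finds the BP_Car in the level and stores it, then creates and displays WBP_HUD.
; Left and right actions set the car's InputDirection to -1 or 1 and reset it on release.
; The drift action only prints a not-implemented message.
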(event `EnhancedInput|/Game/Input/IA_Drift`
  (params (ActionValue :type Boolean) (ElapsedSeconds :type "Float (double-precision)") (TriggeredSeconds :type "Float (double-precision)") (InputAction :type "InputAction Object Reference" :default "/Game/Input/IA_Drift.IA_Drift"))
  (:`Triggered`
    (`KismetSystemLibrary.PrintString` "Drift Not Implemented")))

(event `EnhancedInput|/Game/Input/IA_MoveLeft`
  (params (ActionValue :type Boolean) (ElapsedSeconds :type "Float (double-precision)") (TriggeredSeconds :type "Float (double-precision)") (InputAction :type "InputAction Object Reference" :default "/Game/Input/IA_MoveLeft.IA_MoveLeft"))
  (bind _playeractor (`self.PlayerActor`))
  (:`Started`
    (set `/Game/BP_Car.InputDirection` -1 _playeractor))
  (:`Completed`
    (set `/Game/BP_Car.InputDirection` 0 _playeractor)))

(event `EnhancedInput|/Game/Input/IA_MoveRight`
  (params (ActionValue :type Boolean) (ElapsedSeconds :type "Float (double-precision)") (TriggeredSeconds :type "Float (double-precision)") (InputAction :type "InputAction Object Reference" :default "/Game/Input/IA_MoveRight.IA_MoveRight"))
  (bind _playeractor (`self.PlayerActor`))
  (:`Started`
    (set `/Game/BP_Car.InputDirection` 1 _playeractor))
  (:`Completed`
    (set `/Game/BP_Car.InputDirection` 0 _playeractor)))

(event `self.ReceiveBeginPlay`
  (message `EnhancedInputSubsystemInterface.AddMappingContext` (pcsubsystem `EnhancedInputLocalPlayerSubsystem` (`GameplayStatics.GetPlayerController` 0)) "/Game/Input/IMC_Car.IMC_Car" 0 (struct))
  (bind _returnvalue (`GameplayStatics.GetActorOfClass` "/Game/BP_Car.BP_Car_C"))
  (bind _asbp_car (cast `/Game/BP_Car` _returnvalue))
  (set `self.PlayerActor` _asbp_car)
  (bind _returnvalue_2 (`|CreateWidget` "/Game/WBP_HUD.WBP_HUD_C"))
  (`UserWidget.AddToViewport` _returnvalue_2 0))

(fn `UserConstructionScript`)